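; BP_AI_Enemy is an enemy Blueprint that holds patrol data and tracks whether a BP_Boss actor is nearby.
; On BeginPlay it caches BP_PatrolPoint actors and their count, filtered by PatrolPointsTag when DeterminedPatrolPoints is set, otherwise taking all in the level.
; Sphere overlap events set or clear the ClownNear flag as a BP_Boss enters or leaves.
; The graph contains no movement or behavior logic.
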(event `self.Sphere.OnComponentBeginOverlap`
  (params (OverlappedComponent :type "PrimitiveComponent Object Reference") (OtherActor :type "Actor Object Reference") (OtherComp :type "PrimitiveComponent Object Reference") (OtherBodyIndex :type Integer) (bFromSweep :type Boolean) (SweepResult :type "HitResult Structure (by ref)"))
  (cast `/Game/Characters/Enemy3_Boss/BP_Boss` OtherActor)
  (set `self.Clown Near` true))

(event `self.Sphere.OnComponentEndOverlap`
  (params (OverlappedComponent :type "PrimitiveComponent Object Reference") (OtherActor :type "Actor Object Reference") (OtherComp :type "PrimitiveComponent Object Reference") (OtherBodyIndex :type Integer))
  (cast `/Game/Characters/Enemy3_Boss/BP_Boss` OtherActor)
  (set `self.Clown Near` false))

(event `self.ReceiveBeginPlay`
  ;[0 1 0.09183] Patrol Points
  (if (`self.DeterminedPatrolPoints`)
    (bind _outactors (`GameplayStatics.GetAllActorsOfClassWithTag` "/Game/BP_PatrolPoint.BP_PatrolPoint_C" (`self.PatrolPointsTag`)))
    (bind _output_get (set `self.PatrolPoints` _outactors))
    (set `self.PatrolPointIndexN` (`KismetArrayLibrary.Array_Length` _output_get))
    (else
      (bind _outactors_2 (`GameplayStatics.GetAllActorsOfClass` "/Game/BP_PatrolPoint.BP_PatrolPoint_C"))
      (bind _output_get_2 (set `self.PatrolPoints` _outactors_2))
      (set `self.PatrolPointIndexN` (`KismetArrayLibrary.Array_Length` _output_get_2)))))

(fn `UserConstructionScript`
  (`parent.UserConstructionScript`))