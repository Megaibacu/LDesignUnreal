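; AI controller for enemies that runs BT_Enemy and reacts to perceiving the player, BP_Mc.
; A macro lets stimuli through only when a team-relation data table marks the player hostile to the controlled enemy or boss.
; Noise pulses PlayerSet off and on and stores the player's location, while other stimuli count as sight and set PlayerSpotted.
; Losing either stimulus clears Attacking on the blackboard and on BP_Enemy2 pawns.
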(event `self.ReceiveBeginPlay`
  ;[0.1306 1 0] BehaviorTreeIniciation
  (`self.RunBehaviorTree` "/Game/Characters/Enemy/BT_Enemy.BT_Enemy"))

(event `self.AIPerception.OnTargetPerceptionUpdated`
  (params (Actor :type "Actor Object Reference") (Stimulus :type "AIStimulus Structure"))
  (bind (_age _expirationage _strength _stimuluslocation _receiverlocation _tag _bsuccessfullysensed) (break `AIStimulus` Stimulus))
  ;[1 0 0.8641] StimmuliSeparation
  (bind _asbp_mc (cast `/Game/Characters/MainCharacter/BP_Mc` Actor))
  (set `self.Actor` _asbp_mc)
  (`self.NewMacro_0` _)
  (set `self.Successfully Sensed` _bsuccessfullysensed)
  (if (== _tag "Noise")
    ;[1 0.7933 0.02697] Hear
    (`BlackboardComponent.SetValueAsBool` (`self.Blackboard`) "PlayerSet" false)
    (`KismetSystemLibrary.Delay` 0.1)
    (`BlackboardComponent.SetValueAsBool` (`self.Blackboard`) "PlayerSet" true)
    (`BlackboardComponent.SetValueAsVector` (`self.Blackboard`) "PlayerPos" (`self.K2_GetActorLocation` (`self.Actor`)))
    (if (not (`self.Successfully Sensed`))
      (`BlackboardComponent.SetValueAsBool` (`self.Blackboard`) "Attacking" false)
      (bind _asbp_enemy_2 (cast `/Game/Characters/Enemy2_Eqs/BP_Enemy2` (`self.K2_GetPawn`)))
      (set `/Game/Characters/Enemy2_Eqs/BP_Enemy2.Attacking` false _asbp_enemy_2))
    (else
      ;[0.1102 0.9821 1] Sight
      (`BlackboardComponent.SetValueAsBool` (`self.Blackboard`) "PlayerSpotted" (`self.Successfully Sensed`))
      (if (not (`self.Successfully Sensed`))
        (`BlackboardComponent.SetValueAsBool` (`self.Blackboard`) "Attacking" false)
        (bind _asbp_enemy_2_2 (cast `/Game/Characters/Enemy2_Eqs/BP_Enemy2` (`self.K2_GetPawn`)))
        (set `/Game/Characters/Enemy2_Eqs/BP_Enemy2.Attacking` false _asbp_enemy_2_2)))))

(fn `UserConstructionScript`)