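; AI controller for Enemy2 that runs its behavior tree and tells it when to hide based on the player's weapon.
; BeginPlay caches the BP_Mc player character and starts BT_Enemy2, stopping early if the cast fails.
; The WeaponUpdated event reads the player's WeapontoChange and sets the Hide blackboard key true for any nonzero value, false for zero.
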(event `self.ReceiveBeginPlay`
  ;[0 1 0.07558] Begin play
  (bind _asbp_mc (cast `/Game/Characters/MainCharacter/BP_Mc` (`GameplayStatics.GetPlayerCharacter` 0)))
  (set `self.As BP Mc` _asbp_mc)
  (`self.RunBehaviorTree` "/Game/Characters/Enemy2_Eqs/Ai/BT_Enemy2.BT_Enemy2"))

(event `WeaponUpdated`
  ;[1 0.06741 0] Setting hide
  (if (== (`/Game/Characters/MainCharacter/BP_Mc.WeapontoChange` (`self.As BP Mc`)) 0)
    (`BlackboardComponent.SetValueAsBool` (`self.Blackboard`) "Hide" false)
    (else
      (`BlackboardComponent.SetValueAsBool` (`self.Blackboard`) "Hide" true))))

(fn `UserConstructionScript`
  (`parent.UserConstructionScript`))