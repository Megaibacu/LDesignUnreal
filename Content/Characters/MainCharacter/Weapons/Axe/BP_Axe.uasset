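; BP_Axe is the player's axe weapon, attached to the BP_Mc mesh's SpineSocket on BeginPlay with its hit box collision off.
; A box overlap with a Dummy passes it and its lifebar to BP_Mc, subtracts fixed damage from the widget's Health, then calls KillDummy.
; Each hit disables the box, and a DoOnce with a delayed reset limits repeats.
; The Cloak input toggles an invisible material via FlipFlop.
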(event `InputAction|Cloak`
  (params (Key :type "Key Structure"))
  (:`Pressed`
    (`/Engine/EditorBlueprintResources/StandardMacros.FlipFlop`
      (:`A`
        (`PrimitiveComponent.SetMaterial` (`self.Axe`) 0 "/Game/Characters/MainCharacter/Weapons/Axe/pCube1MatInvisible.pCube1MatInvisible"))
      (:`B`
        (`PrimitiveComponent.SetMaterial` (`self.Axe`) 0 "/Game/Characters/MainCharacter/Weapons/Axe/pCube1Mat.pCube1Mat")))))

(event `self.ReceiveBeginPlay`
  (bind _asbp_mc (cast `/Game/Characters/MainCharacter/BP_Mc` (`GameplayStatics.GetPlayerPawn` 0)))
  (set `self.BP Mc` _asbp_mc)
  (`self.K2_AttachToComponent` (`Character.Mesh` _asbp_mc) "SpineSocket" "KeepRelative" "KeepRelative" "KeepRelative")
  (`PrimitiveComponent.SetCollisionEnabled` (`self.Box`) "NoCollision"))

(event `self.Box.OnComponentBeginOverlap`
  (params (OverlappedComponent :type "PrimitiveComponent Object Reference") (OtherActor :type "Actor Object Reference") (OtherComp :type "PrimitiveComponent Object Reference") (OtherBodyIndex :type Integer) (bFromSweep :type Boolean) (SweepResult :type "HitResult Structure (by ref)"))
  (`/Engine/EditorBlueprintResources/StandardMacros.DoOnce` false :!label _label
    (:`Completed`
      (bind _asdummy (cast `/Game/Characters/PracticeDummy/source/Dummy` OtherActor))
      (set `/Game/Characters/MainCharacter/BP_Mc.As Dummy` _asdummy (`self.BP Mc`))
      (bind _asdummy_lifebar (cast `/Game/Characters/PracticeDummy/source/DummyLifebar` (`WidgetComponent.GetWidget` (`/Game/Characters/PracticeDummy/source/Dummy.Widget` _asdummy))))
      (set `/Game/Characters/MainCharacter/BP_Mc.As Dummy Lifebar` _asdummy_lifebar (`self.BP Mc`))
      (set `/Game/Characters/PracticeDummy/source/DummyLifebar.Health` (- (`/Game/Characters/PracticeDummy/source/DummyLifebar.Health` _asdummy_lifebar) 25.0) _asdummy_lifebar)
      (bind _asbp_mc (cast `/Game/Characters/MainCharacter/BP_Mc` (`GameplayStatics.GetPlayerPawn` 0)))
      (`/Game/Characters/MainCharacter/BP_Mc.KillDummy` _asbp_mc)
      (`PrimitiveComponent.SetCollisionEnabled` (`self.Box`) "NoCollision")
      (`KismetSystemLibrary.Delay` 1.0)
      (goto _label :!via `Reset`))))

(fn `UserConstructionScript`)